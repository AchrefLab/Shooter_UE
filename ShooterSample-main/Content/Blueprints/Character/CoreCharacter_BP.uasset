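; CoreCharacter_BP is a first-person player character that moves, jumps, looks around and fires projectiles.
; Axis inputs drive movement along the actor's forward and right vectors, while mouse yaw and pitch are scaled by MouseSensitivity.
; Fire spawns a CoreProjectile_BP at the FPGun's projectile socket, rotated to the base aim rotation, with the character as owner and instigator.
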(event `InputAxis|MoveForward` :consume false :overrideparent false
  (params (AxisValue :type "Float (single-precision)"))
  ;[1 1 1] This part is to move around the world (Forwards and Right)
  (`self.AddMovementInput` (`self.GetActorForwardVector`) AxisValue))

(event `InputAction|Jump`
  (params (Key :type "Key Structure"))
  ;[1 1 1] Input for jumping
  (:`Pressed`
    (`self.Jump`))
  (:`Released`
    (`self.StopJumping`)))

(event `InputAxis|MoveRight` :consume false :overrideparent false
  (params (AxisValue :type "Float (single-precision)"))
  ;[1 1 1] This part is to move around the world (Forwards and Right)
  (`self.AddMovementInput` (`self.GetActorRightVector`) AxisValue))

(event `InputAction|Fire`
  (params (Key :type "Key Structure"))
  (:`Pressed`
    (`|SpawnActorFromClass` "/Game/Blueprints/Projectiles/CoreProjectile_BP.CoreProjectile_BP_C" (`KismetMathLibrary.MakeTransform` (`SceneComponent.GetSocketLocation` (`self.FP_Gun`) "Projectile_Socket") (`self.GetBaseAimRotation`)) "AlwaysSpawn" "OverrideRootScale" self self)))

(event `InputAxis|Turn` :overrideparent false
  (params (AxisValue :type "Float (single-precision)"))
  ;[1 1 1] This part is to move the screen and see around
  ;;[1 1 1] Mouse X
  (`self.AddControllerYawInput` (* AxisValue (`self.MouseSensitivity`))))

(event `InputAxis|LookUp` :overrideparent false
  (params (AxisValue :type "Float (single-precision)"))
  ;[1 1 1] This part is to move the screen and see around
  ;;[1 1 1] Mouse Y
  (`self.AddControllerPitchInput` (* AxisValue (`self.MouseSensitivity`))))

(fn `UserConstructionScript`)