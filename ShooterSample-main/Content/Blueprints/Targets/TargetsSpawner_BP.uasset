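; Spawner actor that keeps creating CoreTargets_BP targets at random points inside its Sphere component.
; Tick feeds a Delay of random 0.5 to 1.5 second length, which throttles spawning because repeat calls are ignored while it runs.
; Each location is a random direction times a random distance up to the scaled radius, so targets cluster toward the center.
; Targets take the spawner's rotation, with player character 0 as owner and instigator.
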(event `self.ReceiveTick`
  (params (DeltaSeconds :type "Float (single-precision)"))
  (bind _returnvalue (`GameplayStatics.GetPlayerCharacter` 0))
  ;[1 1 1] Random delay between 1.5 and 0.5
  (`KismetSystemLibrary.Delay` (+ (`KismetMathLibrary.RandomFloat`) 0.5))
  (`|SpawnActorFromClass` "/Game/Blueprints/Targets/CoreTargets_BP.CoreTargets_BP_C" (`KismetMathLibrary.MakeTransform` (+ (* (`KismetMathLibrary.RandomUnitVector`) (`KismetMathLibrary.RandomFloatInRange` 0.0 (`SphereComponent.GetScaledSphereRadius` (`self.Sphere`)))) (`self.K2_GetActorLocation`)) (`self.K2_GetActorRotation`)) "Undefined" "OverrideRootScale" _returnvalue _returnvalue))

(fn `UserConstructionScript`)